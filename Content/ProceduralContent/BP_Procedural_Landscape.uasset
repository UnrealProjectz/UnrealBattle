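; Procedural landscape prototype that, on BeginPlay, lays out a grid of points from its ProceduralMesh location and shows them as debug points.
; Make2dArrayAndPlane stores the grid in a flattened vector array, adding an extra entry at each column start and printing indices.
; 2dArrayGet highlights one stored point in green, indexing only by column position and column length.
; Mesh section creation is unconnected and Set2dArray is empty, so no mesh is generated.
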(event `self.ReceiveBeginPlay`
  (`self.Make 2d array and plane` 15 15 (`self.Location`))
  (`self.2d array Get` 15 15 4 4 (`self.Location`)))

(fn `2d array Get`
  (params (Row_Length :type Integer) (Col_Legth :type Integer) (Row_Position :type Integer) (Col_Position :type Integer) (Stroage_Vector :type "Array of Vector Structure"))
  (`KismetSystemLibrary.DrawDebugPoint` (`|GetArrayItem` Stroage_Vector (* (+ Col_Position 1) Col_Legth)) 11.0 (struct :`R` 0.021328 :`G` 1.0 :`A` 1.0) 100.0))

(fn `Make 2d array and plane`
  (params (Row_Length :type Integer) (Col_Length :type Integer) (StorageVector :type "Array of Vector Structure"))
  (`|ExecutionSequence`
    (:`then_0`
      (for _index (range Col_Length)
        (bind _returnvalue (+ (`SceneComponent.K2_GetComponentLocation` (`self.ProceduralMesh`)) (* (10.0 0.0 0.0) _index)))
        (`KismetArrayLibrary.Array_Add` StorageVector _returnvalue)
        (`KismetSystemLibrary.DrawDebugPoint` _returnvalue 10.0 (struct :`R` 1.0 :`B` 0.140109 :`A` 1.0) 1000.0)
        (for _index_2 (range Row_Length)
          (bind _returnvalue_2 (+ _returnvalue (* (0.0 10.0 0.0) _index_2)))
          (bind _returnvalue_3 (`KismetArrayLibrary.Array_Add` StorageVector _returnvalue_2))
          (`KismetSystemLibrary.DrawDebugPoint` _returnvalue_2 10.0 (struct :`R` 1.0 :`B` 0.224284 :`A` 1.0) 1000.0)
          (`KismetSystemLibrary.PrintString` (`KismetStringLibrary.Conv_IntToString` (+ _returnvalue_3 1)) true true (struct :`G` 0.66 :`B` 1.0 :`A` 1.0) 100.0))))))

(fn `Set 2d array`)

(fn `UserConstructionScript`)